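; Behavior Tree task that gradually heals the AI-controlled pawn until its health reaches the HealToMin threshold.
; It finds the pawn's CHHealthComponent, then loops through a latent Delay, applying a fixed heal after each wait.
; The task finishes successfully once health is at or above the threshold, and calls FinishAbort if the component is missing.
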(event `self.ReceiveExecuteAI`
  (params (OwnerController :type "AIController Object Reference") (ControlledPawn :type "Pawn Object Reference"))
  (bind _output_get (set `self.HealthComp` (`Actor.GetComponentByClass` ControlledPawn "/Script/Coop.CHHealthComponent")))
  (`/Engine/EditorBlueprintResources/StandardMacros.IsValid` _output_get
    (:`Is Valid`
      (if (< (`CHHealthComponent.Health` (`self.HealthComp`)) (`self.HealToMin`)) :!label _label
        (`KismetSystemLibrary.Delay` 2.0)
        (`CHHealthComponent.Heal` (`self.HealthComp`) 10.0)
        (goto _label)
        (else
          (`self.FinishExecute` true))))
    (:`Is Not Valid`
      (`self.FinishAbort`))))