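; Behavior tree service that selects the nearest living, non-friendly actor as the AI pawn's target.
; Each AI tick, it scans the sight sense's known perceived actors from the pawn's AIPerceptionComponent, filtering by IsFrendly and CHHealthComponent health.
; It writes the closest match to a configurable blackboard key.
; BestActor is not cleared between scans, so the last pick can carry over when nothing qualifies.
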(event `self.ReceiveTickAI`
  (params (OwnerController :type "AIController Object Reference") (ControlledPawn :type "Pawn Object Reference") (DeltaSeconds :type "Float (single-precision)"))
  (set `self.NearestTargetDist` 4.0896499921872486e+18)
  (for _array_element (`AIPerceptionComponent.GetKnownPerceivedActors` (`Actor.GetComponentByClass` ControlledPawn "/Script/AIModule.AIPerceptionComponent") "/Script/AIModule.AISense_Sight")
    (if (and (not (`CHHealthComponent.IsFrendly` ControlledPawn _array_element)) (> (`CHHealthComponent.Health` (`Actor.GetComponentByClass` _array_element "/Script/Coop.CHHealthComponent")) 0.0))
      (bind _returnvalue (`KismetMathLibrary.VSize` (- (`Actor.K2_GetActorLocation` _array_element) (`Actor.K2_GetActorLocation` ControlledPawn))))
      (if (< _returnvalue (`self.NearestTargetDist`))
        (set `self.NearestTargetDist` _returnvalue)
        (set `self.BestActor` _array_element))))
  (`BTFunctionLibrary.SetBlackboardValueAsObject` (`self.BlackbordKey`) (`self.BestActor`)))