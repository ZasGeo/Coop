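; Game mode Blueprint that awards kill score and spawns tracker bots.
; On BeginPlay it binds to the actor-killed event, adding a point to the killer's CHPlayerState and printing the new score.
; SpawnNewBot, which nothing in this graph calls, runs the EQS_FindSpawnLocation query in random-best-25% mode.
; On query success, it draws a debug sphere and attempts to spawn a BP_TrackerBot at each returned location, adjusting for collisions.
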(event `self.ReceiveBeginPlay`
  (add `self.OnActorKilled` (delegate `OnActorKilled_Event`)))

(event `OnActorKilled_Event` :!signature `self.OnActorKilled`
  (params (VictimActor :type "Actor Object Reference") (KillerActor :type "Actor Object Reference") (KillerController :type "Controller Object Reference"))
  (`/Engine/EditorBlueprintResources/StandardMacros.IsValid` KillerController
    (:`Is Valid`
      (bind _aschplayer_state (cast `CHPlayerState` (`Pawn.PlayerState` (`Controller.K2_GetPawn` KillerController))))
      (`CHPlayerState.AddScore` _aschplayer_state 1.0)
      (`KismetSystemLibrary.PrintString` (`KismetStringLibrary.Conv_DoubleToString` (`PlayerState.Score` _aschplayer_state))))))

(event `self.SpawnNewBot`
  (bind _returnvalue (`EnvQueryManager.RunEQSQuery` "/Game/Blueprints/EQS/EQS_FindSpawnLocation.EQS_FindSpawnLocation" self "RandomBest25Pct"))
  (add `EnvQueryInstanceBlueprintWrapper.OnQueryFinishedEvent` _returnvalue (delegate `OnQueryFinishedEvent`)))

(event `OnQueryFinishedEvent`
  (params (QueryInstance :type "EnvQueryInstanceBlueprintWrapper Object Reference") (QueryStatus :type "EEnvQueryStatus Enum" :default "Processing"))
  (switch `EEnvQueryStatus` QueryStatus
    (:`Success`
      (bind _resultlocations (`EnvQueryInstanceBlueprintWrapper.GetQueryResultsAsLocations` QueryInstance))
      (for _array_element _resultlocations
        (`KismetSystemLibrary.DrawDebugSphere` _array_element 50.0 12 (struct :`R` 1.0 :`G` 0.835401 :`A` 1.0) 2.0 2.0)
        (`|SpawnActorFromClass` "/Game/Blueprints/BP_TrackerBot.BP_TrackerBot_C" (`KismetMathLibrary.MakeTransform` _array_element) "AdjustIfPossibleButDontSpawnIfColliding" "OverrideRootScale" null null)))))

(fn `UserConstructionScript`)